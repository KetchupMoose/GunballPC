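; Multiplayer player controller for Gunball that requests a pawn spawn from the game mode after login and manages match UI.
; Score, scorer and win events update the HUD held by the Steam game instance.
; It creates and dismisses the end-of-match screen, switching input modes, and forwards rematch and map-change requests to game state or mode.
; A rep-notify hides that screen on clients, but its flag setter and the HUD creation code are disconnected.
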(event `SpawnPawnOnServer`
  (bind _asmy_gunball_game_mode (cast `/Game/GunballMapBP/MyGunballGameMode` (`GameplayStatics.GetGameMode`)))
  (`/Game/GunballMapBP/MyGunballGameMode.RespawnPlayerEvent` _asmy_gunball_game_mode self))

(event `SpawnPawnForPlayer`
  (`KismetSystemLibrary.PrintString` "BeginPlayForPC")
  (`self.SpawnPawnOnServer`))

(event `self.ReceiveBeginPlay`)

(event `ClientPostLogin`
  ;[1 1 1] after login, set up UI and spawn the player
  (`self.SpawnPawnForPlayer`))

(event `self.ReceiveEndPlay`
  (params (EndPlayReason :type "EEndPlayReason Enum" :default "Destroyed"))
  ;[1 1 1] remove hud on end of session
  (`Widget.RemoveFromParent` (`self.PlayerHUD`)))

(event `PC_Rematch`
  (bind _asgs_mp (cast `/Game/Multiplayer/Blueprints/GS_MP` (`GameplayStatics.GetGameState`)))
  (`/Game/Multiplayer/Blueprints/GS_MP.GS_Trigger_Remove_EndMatchHud` _asgs_mp))

(event `ReplicatedRematch`
  (`self.PC_DestroyEndMatchHud`)
  (`/Engine/EditorBlueprintResources/ActorMacros.Switch Has Authority`))

(event `TellGameModeChangeMap`
  (bind _asmy_gunball_game_mode (cast `/Game/GunballMapBP/MyGunballGameMode` (`GameplayStatics.GetGameMode`)))
  (`/Game/GunballMapBP/MyGunballGameMode.GameModeChangeMap` _asmy_gunball_game_mode))

(event `PC_Update_Huds`
  (params (PlayerScored :type Integer))
  (if (== PlayerScored 0)
    (bind _asgi_mp_steam (cast `/Game/Multiplayer/Blueprints/GI_MP_STEAM` (`GameplayStatics.GetGameInstance`)))
    (`/Game/Multiplayer/Widget/W_MP_HUD.SetGoalScorerText` (`/Game/Multiplayer/Blueprints/GI_MP_STEAM.MPHud` _asgi_mp_steam) "Oops Own Goal!")
    (else
      (cast `/Game/Multiplayer/Blueprints/GS_MP` (`GameplayStatics.GetGameState`))
      (bind _asgi_mp_steam_2 (cast `/Game/Multiplayer/Blueprints/GI_MP_STEAM` (`GameplayStatics.GetGameInstance`)))
      (bind _mphud (`/Game/Multiplayer/Blueprints/GI_MP_STEAM.MPHud` _asgi_mp_steam_2))
      (`/Game/Multiplayer/Widget/W_MP_HUD.SetGoalScorerText` _mphud (`KismetTextLibrary.Conv_StringToText` (`PlayerState.PlayerName` (`KismetArrayLibrary.Array_Get` (`/Game/Multiplayer/Widget/W_MP_HUD.SortedArrrayOfPlayerStates` _mphud) (- PlayerScored 1))))))))

(event `PC_UpdateHudGoalLabel`
  (params (TeamScored :type Integer))
  (bind _asgi_mp_steam (cast `/Game/Multiplayer/Blueprints/GI_MP_STEAM` (`GameplayStatics.GetGameInstance`)))
  (`/Game/Multiplayer/Widget/W_MP_HUD.SetGoalText` (`/Game/Multiplayer/Blueprints/GI_MP_STEAM.MPHud` _asgi_mp_steam) TeamScored false)
  (`KismetSystemLibrary.K2_SetTimer` null "ResetScoreLabel" 0.8))

(event `ResetScoreLabel`
  (bind _asgi_mp_steam (cast `/Game/Multiplayer/Blueprints/GI_MP_STEAM` (`GameplayStatics.GetGameInstance`)))
  (`/Game/Multiplayer/Widget/W_MP_HUD.SetGoalText` (`/Game/Multiplayer/Blueprints/GI_MP_STEAM.MPHud` _asgi_mp_steam) 1 true))

(event `PC_Set_Win_Label`
  (params (TeamWon :type Integer))
  (bind _asgi_mp_steam (cast `/Game/Multiplayer/Blueprints/GI_MP_STEAM` (`GameplayStatics.GetGameInstance`)))
  (`/Game/Multiplayer/Widget/W_MP_HUD.SetWinText` (`/Game/Multiplayer/Blueprints/GI_MP_STEAM.MPHud` _asgi_mp_steam) TeamWon))

(event `PC_CreateEndOfMatchHud`
  (bind _returnvalue (`|CreateWidget` "/Game/Multiplayer/Widget/W_EndOfMatchScreen.W_EndOfMatchScreen_C" self))
  (bind _output_get (set `self.EndOfMatchHUD` _returnvalue))
  (set `/Game/Multiplayer/Widget/W_EndOfMatchScreen.OwningPlayerHUD` self _output_get)
  (`UserWidget.AddToViewport` _output_get 0)
  (`WidgetBlueprintLibrary.SetInputMode_UIOnlyEx` self (`self.EndOfMatchHUD`))
  (set `self.bShowMouseCursor` true)
  (`/Game/Multiplayer/Widget/W_EndOfMatchScreen.SetEndOfMatchText` (`self.EndOfMatchHUD`)))

(event `PCSetInputMode`
  (`WidgetBlueprintLibrary.SetInputMode_GameOnly` self)
  (set `self.bShowMouseCursor` false))

(event `PC_DestroyEndMatchHud`
  (bind _asgi_mp_steam (cast `/Game/Multiplayer/Blueprints/GI_MP_STEAM` (`GameplayStatics.GetGameInstance`)))
  (`Widget.RemoveFromParent` (`/Game/Multiplayer/Blueprints/GI_MP_STEAM.EndOfMatchHUD` _asgi_mp_steam))
  (`WidgetBlueprintLibrary.SetInputMode_GameOnly` self)
  (set `self.bShowMouseCursor` false))

(event `PC_Initiate_ServerHudDestroy`
  (bind _asmy_gunball_game_mode (cast `/Game/GunballMapBP/MyGunballGameMode` (`GameplayStatics.GetGameMode`)))
  (`/Game/GunballMapBP/MyGunballGameMode.TellGameStateToSetPCInputMode` _asmy_gunball_game_mode))

(event `PC_RPCToServer`
  (`/Engine/EditorBlueprintResources/ActorMacros.Switch Has Authority`
    (:`Authority`
      _)
    (:`Remote`
      _))
  (bind _asgi_mp_steam (cast `/Game/Multiplayer/Blueprints/GI_MP_STEAM` (`GameplayStatics.GetGameInstance`)))
  (`/Game/Multiplayer/Blueprints/GI_MP_STEAM.GI_DismissEoMHuds` _asgi_mp_steam (`/Game/Multiplayer/Widget/W_MP_HUD.OwningPlayer` (`/Game/Multiplayer/Blueprints/GI_MP_STEAM.MPHud` _asgi_mp_steam))))

(fn `OnRep_tellPlayerGameRestarting`
  (bind _returnvalue (`GameplayStatics.GetPlayerController` 0))
  (`/Engine/EditorBlueprintResources/ActorMacros.Switch Has Authority`
    (:`Remote`
      (if (`self.tellPlayerGameRestarting`)
        (bind _foundwidgets (`WidgetBlueprintLibrary.GetAllWidgetsOfClass` "/Game/Multiplayer/Widget/W_EndOfMatchScreen.W_EndOfMatchScreen_C"))
        (for _array_element _foundwidgets
          (`Widget.SetVisibility` _array_element "Hidden"))
        (`WidgetBlueprintLibrary.SetInputMode_GameOnly` _returnvalue)
        (set `PlayerController.bShowMouseCursor` false _returnvalue)
        (set `self.tellPlayerGameRestarting` false)))))

(fn `SetupGameHud`)

(fn `UserConstructionScript`)