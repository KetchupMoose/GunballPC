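; Multiplayer game state that tracks replicated player and team scores and drives each machine's match feedback.
; Score RepNotifies update HUDs and scoreboards through the local PC_MP, and a team reaching MaxScore triggers the win label and end-of-match screen via GI_MP_STEAM.
; Player score changes can move CurrentCrown, toggling tagged crown meshes on characters to mark the leader.
; A replicated reset flag dismisses the end-of-match HUD.
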(event `UpdateClientHudsWithScore`
  (params (PlayerScored :type Integer))
  (bind _aspc_mp (cast `/Game/Multiplayer/Blueprints/PC_MP` (`GameplayStatics.GetPlayerController` 0)))
  (`/Game/Multiplayer/Blueprints/PC_MP.PC_Update_Huds` _aspc_mp PlayerScored))

(event `GS_TellPCSToRemoveEOMHud`
  (bind _aspc_mp (cast `/Game/Multiplayer/Blueprints/PC_MP` (`GameplayStatics.GetPlayerController` 0)))
  (`/Game/Multiplayer/Blueprints/PC_MP.PC_DestroyEndMatchHud` _aspc_mp))

(event `UpdateScoreboards`
  (bind _outactors (`GameplayStatics.GetAllActorsOfClass` "/Game/Scoreboard.Scoreboard_C"))
  (for _array_element _outactors
    (`/Game/Scoreboard.UpdateScoreboard` _array_element)))

(event `AddTeamGoalLabelToMPHud`
  (params (TeamScored :type Integer))
  (bind _aspc_mp (cast `/Game/Multiplayer/Blueprints/PC_MP` (`GameplayStatics.GetPlayerController` 0)))
  (`/Game/Multiplayer/Blueprints/PC_MP.PC_UpdateHudGoalLabel` _aspc_mp TeamScored))

(event `GS_SetWinLabel`
  (params (WinningTeam :type Integer))
  (bind _aspc_mp (cast `/Game/Multiplayer/Blueprints/PC_MP` (`GameplayStatics.GetPlayerController` 0)))
  (`/Game/Multiplayer/Blueprints/PC_MP.PC_Set_Win_Label` _aspc_mp WinningTeam))

(event `GS_Trigger_End_MatchHUD`
  (bind _asgi_mp_steam (cast `/Game/Multiplayer/Blueprints/GI_MP_STEAM` (`GameplayStatics.GetGameInstance`)))
  (`/Game/Multiplayer/Blueprints/GI_MP_STEAM.CreateEndOfMatchScreen` _asgi_mp_steam))

(event `GS_Trigger_Remove_EndMatchHud`
  (bind _asgi_mp_steam (cast `/Game/Multiplayer/Blueprints/GI_MP_STEAM` (`GameplayStatics.GetGameInstance`)))
  (`/Game/Multiplayer/Blueprints/GI_MP_STEAM.GI_DismissEoMHuds` _asgi_mp_steam null))

(event `GSRemoveHud`
  (`self.ClientRemovesHud`))

(event `ClientRemovesHud`
  (bind _aspc_mp (cast `/Game/Multiplayer/Blueprints/PC_MP` (`GameplayStatics.GetPlayerController` 0)))
  (`/Game/Multiplayer/Blueprints/PC_MP.PCSetInputMode` _aspc_mp))

(event `AwardCrowns`
  (params (PlayerCrown :type Integer))
  (bind _outactors (`GameplayStatics.GetAllActorsOfClass` "/Game/FirstPersonBP/Blueprints/FirstPersonCharacter.FirstPersonCharacter_C"))
  (for _array_element _outactors
    (bind _asps_mp (cast `/Game/Multiplayer/Blueprints/PS_MP` (`Pawn.PlayerState` _array_element)))
    (bind _playernumber (`/Game/Multiplayer/Blueprints/PS_MP.Get The PlayerNumber` _asps_mp))
    ;[1 1 1] crown a new player, remove crowns from other players
    (if (== PlayerCrown _playernumber)
      (bind _item (`KismetArrayLibrary.Array_Get` (`self.GetComponentsByTag` _array_element "/Script/Engine.StaticMeshComponent" "crown")))
      (`SceneComponent.SetHiddenInGame` _item false false)
      (else
        (`SceneComponent.SetHiddenInGame` _item true false)))))

(fn `CheckForWin`
  (if (== (`self.Team1Score`) (`self.maxScore`))
    (`self.GS_SetWinLabel` 1)
    (`self.GS_Trigger_End_MatchHUD` :!label _label)
    (elif (== (`self.Team2Score`) (`self.maxScore`))
      (`self.GS_SetWinLabel` 2)
      (goto _label))))

(fn `GetThePlayerArray`
  (returns (returningPlayerArray :type "Array of PlayerState Object Reference"))
  (return (`self.PlayerArray`)))

(fn `GiveNewPlayerCrown`
  (params (PlayerScore :type Integer) (PlayerNumber :type Integer))
  (if (== PlayerNumber (`self.currentCrown`))
    _
    (elif (>= PlayerScore (`.MaxValue` (`KismetMathLibrary.MaxOfIntArray` (`|MakeArray` (`self.Player1Score`) (`self.Player2Score`) (`self.Player3Score`) (`self.Player4Score`)))))
      ;[1 1 1] crown a new player, remove crowns from other players
      (bind _outactors (`GameplayStatics.GetAllActorsOfClass` "/Game/FirstPersonBP/Blueprints/FirstPersonCharacter.FirstPersonCharacter_C" :!label _label))
      (for _array_element _outactors
        (bind _asps_mp (cast `/Game/Multiplayer/Blueprints/PS_MP` (`Pawn.PlayerState` _array_element)))
        (bind _playernumber (`/Game/Multiplayer/Blueprints/PS_MP.Get The PlayerNumber` _asps_mp))
        (if (== PlayerNumber _playernumber)
          (bind _item (`KismetArrayLibrary.Array_Get` (`self.GetComponentsByTag` _array_element "/Script/Engine.StaticMeshComponent" "crown")))
          (`SceneComponent.SetHiddenInGame` _item false false)
          (set `self.currentCrown` PlayerNumber)
          (else
            (`SceneComponent.SetHiddenInGame` _item true false))))
      (elif (== (`self.currentCrown`) 0)
        (goto _label)))))

(fn `OnRep_currentCrown`
  (`self.AwardCrowns` (`self.currentCrown`)))

(fn `OnRep_gameRestarting`)

(fn `OnRep_Player0Score`
  (`self.UpdateClientHudsWithScore` 0))

(fn `OnRep_Player1Score`
  (`self.UpdateClientHudsWithScore` 1)
  (`self.GiveNewPlayerCrown` (`self.Player1Score`) 1))

(fn `OnRep_Player2Score`
  (`self.UpdateClientHudsWithScore` 2)
  (`self.GiveNewPlayerCrown` (`self.Player2Score`) 2))

(fn `OnRep_Player3Score`
  (`self.UpdateClientHudsWithScore` 3)
  (`self.GiveNewPlayerCrown` (`self.Player3Score`) 3))

(fn `OnRep_Player4Score`
  (`self.UpdateClientHudsWithScore` 4)
  (`self.GiveNewPlayerCrown` (`self.Player4Score`) 4))

(fn `OnRep_resetEOMScreen`
  (if (`self.resetEOMScreen`)
    (`self.GS_TellPCSToRemoveEOMHud`)))

(fn `OnRep_Team1Score`
  (`self.UpdateScoreboards`)
  (`self.AddTeamGoalLabelToMPHud` 1)
  (`self.CheckForWin`))

(fn `OnRep_Team2Score`
  (`self.UpdateScoreboards`)
  (`self.AddTeamGoalLabelToMPHud` 2)
  (`self.CheckForWin`))

(fn `UserConstructionScript`)