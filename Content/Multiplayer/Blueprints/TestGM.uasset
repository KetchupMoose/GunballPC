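; Multiplayer game mode that handles player login and respawning for two player sides.
; On login it records the controller, sorts PlayerStarts by the "player1" tag, numbers the PS_MP state for consistent scoreboard order, then calls ClientPostLogin on PC_MP.
; RespawnPlayerEvent destroys the pawn, then spawns and possesses a FirstPersonCharacter at the first start for that side.
; The first PlayerArray entry uses player 1's start; everyone else uses player 2's.
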(event `self.K2_PostLogin`
  (params (NewPlayer :type "PlayerController Object Reference"))
  (`KismetArrayLibrary.Array_Add` (`self.playerControllerList`) NewPlayer)
  (`/Engine/EditorBlueprintResources/ActorMacros.Switch Has Authority`
    (:`Authority`
      (bind _outactors (`GameplayStatics.GetAllActorsOfClass` "/Script/Engine.PlayerStart"))
      (for _array_element _outactors
        (bind _asplayer_start (cast `PlayerStart` _array_element))
        (if (== (`PlayerStart.PlayerStartTag` _asplayer_start) "player1")
          (`KismetArrayLibrary.Array_AddUnique` (`self.player1Start`) _asplayer_start)
          (else
            (`KismetArrayLibrary.Array_AddUnique` (`self.player2Start`) _asplayer_start))))
      (bind _asps_mp (cast `/Game/Multiplayer/Blueprints/PS_MP` (`Controller.PlayerState` NewPlayer)))
      ;[1 1 1] verifies scoreboard will be in same order for all players
      (set `/Game/Multiplayer/Blueprints/PS_MP.playerNumber` (`KismetArrayLibrary.Array_Length` (`GameStateBase.PlayerArray` (`GameplayStatics.GetGameState`))) _asps_mp)
      (bind _aspc_mp (cast `/Game/Multiplayer/Blueprints/PC_MP` NewPlayer))
      (`/Game/Multiplayer/Blueprints/PC_MP.ClientPostLogin` _aspc_mp))))

(event `RespawnPlayerEvent`
  (params (playerController :type "PlayerController Object Reference"))
  ;[1 1 1] respawn player 1 and 2 at respectivre spawns
  (`self.K2_DestroyActor` (`Controller.K2_GetPawn` playerController))
  (if (== (`PlayerState.PlayerId` (`Controller.PlayerState` playerController)) (`PlayerState.PlayerId` (`KismetArrayLibrary.Array_Get` (`GameStateBase.PlayerArray` (`GameplayStatics.GetGameState`)))))
    (bind _returnvalue (`|SpawnActorFromClass` "/Game/FirstPersonBP/Blueprints/FirstPersonCharacter.FirstPersonCharacter_C" (`self.GetTransform` (`KismetArrayLibrary.Array_Get` (`self.player1Start`))) "AdjustIfPossibleButAlwaysSpawn" "OverrideRootScale"))
    (`Controller.Possess` playerController _returnvalue)
    (else
      (bind _returnvalue_2 (`|SpawnActorFromClass` "/Game/FirstPersonBP/Blueprints/FirstPersonCharacter.FirstPersonCharacter_C" (`self.GetTransform` (`KismetArrayLibrary.Array_Get` (`self.player2Start`))) "AdjustIfPossibleButAlwaysSpawn" "OverrideRootScale"))
      (`Controller.Possess` playerController _returnvalue_2))))

(fn `UserConstructionScript`)