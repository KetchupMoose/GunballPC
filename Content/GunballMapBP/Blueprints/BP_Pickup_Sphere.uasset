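; BP_Pickup_Sphere is a physics sphere for Gunball that can be picked up, dropped and scored in goals.
; Pickup turns off physics and attaches the root to the given component, while Drop re-enables physics and detaches it, both keeping world transform.
; Hitting a Goal passes that goal's Player to the GunballGameModeBase's CalculateScore, then destroys the sphere.
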(event `/Game/GunballMapBP/Blueprints/PickupActorInterface.Pickup`
  (params (AttachTo :type "SceneComponent Object Reference"))
  (`PrimitiveComponent.SetSimulatePhysics` (`self.StaticMeshComponent`) false)
  (`SceneComponent.K2_AttachToComponent` (`self.K2_GetRootComponent`) AttachTo "None" "KeepWorld" "KeepWorld" "KeepWorld" false))

(event `/Game/GunballMapBP/Blueprints/PickupActorInterface.Drop`
  (`PrimitiveComponent.SetSimulatePhysics` (`self.StaticMeshComponent`) true)
  (`self.K2_DetachFromActor` "KeepWorld" "KeepWorld" "KeepWorld"))

(event `self.ReceiveHit`
  (params (MyComp :type "PrimitiveComponent Object Reference") (Other :type "Actor Object Reference") (OtherComp :type "PrimitiveComponent Object Reference") (bSelfMoved :type Boolean) (HitLocation :type "Vector Structure") (HitNormal :type "Vector Structure") (NormalImpulse :type "Vector Structure") (Hit :type "HitResult Structure (by ref)"))
  ;[1 1 1] Find which goal
  (if (`KismetMathLibrary.ClassIsChildOf` (`GameplayStatics.GetObjectClass` Other) "/Game/Goal.Goal_C")
    (bind _asgoal (cast `/Game/Goal` Other))
    (bind _asgunball_game_mode_base (cast `GunballGameModeBase` (`GameplayStatics.GetGameMode`)))
    ;[1 1 1] Create function for setting player score
    (`GunballGameModeBase.CalculateScore` _asgunball_game_mode_base (`/Game/Goal.Player` _asgoal))
    (`self.K2_DestroyActor`)))

(fn `UserConstructionScript`)